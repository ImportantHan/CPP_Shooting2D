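; Player pawn Blueprint with helper functions for frame-rate-independent movement in the plane of the actor's right and up vectors.
; GetDirection normalizes horizontal and vertical values along those axes, and Translate offsets the location by direction, speed and world delta seconds without sweeping.
; The movement call is disconnected from Tick, so it never runs as the graph stands.
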(event EventBeginPlay)

(event Collision|EventActorBeginOverlap
  (params (OtherActor :type Actor%20Object%20Reference)))

(event EventTick
  (params (DeltaSeconds :type Float%20%28single-precision%29)))

(fn ConstructionScript)

(fn GetDirection
  (return (Math|Vector|Normalize (+ (* (Input|AxisValues|GetHorizontal) (Transformation|GetActorRightVector)) (* (Input|AxisValues|GetVertical) (Transformation|GetActorUpVector))))))

(fn Translate
  (params (Direction :type Vector) (Speed :type Float%20%28double-precision%29))
  (Transformation|SetActorLocation (+ (Transformation|GetActorLocation) (* Direction Speed (Utilities|Time|GetWorldDeltaSeconds))) false false))